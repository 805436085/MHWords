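; MHGameMode is a game mode Blueprint that sets up and starts a fight between a player and a monster at BeginPlay.
; Two helper functions (创建玩家, 创建怪物) spawn and store BP_Player and BP_Monster, printing an error if either is invalid.
; After a two-second delay it adds an MHMainWindow widget to the viewport, passes it to the player, and calls the player's Fight with both actors.
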(event `self.ReceiveBeginPlay`
  (bind _player (`self.Player`))
  (`self.创建玩家`)
  (`self.创建怪物`)
  (`KismetSystemLibrary.Delay` 2.0)
  (bind _returnvalue (`|CreateWidget` "/Game/HUD/MHMainWindow.MHMainWindow_C"))
  (`UserWidget.AddToViewport` _returnvalue 0)
  (set `/Game/BluePrint/BP_Player.mainwindow` _returnvalue (`self.Player`))
  (`MHCharacterBase.fight` _player _player (`self.Monster`)))

(fn `UserConstructionScript`)

(fn `创建怪物`
  (bind _returnvalue (`|SpawnActorFromClass` "/Game/BluePrint/BP_Monster.BP_Monster_C" (`self.Spawn Transform`) "Undefined" "OverrideRootScale" null null))
  (bind _output_get (set `self.Monster` _returnvalue))
  (`/Engine/EditorBlueprintResources/StandardMacros.IsValid` _output_get
    (:`Is Valid`
      _)
    (:`Is Not Valid`
      (`KismetSystemLibrary.PrintString` "create monster error")))
  (return))

(fn `创建玩家`
  (bind _returnvalue (`|SpawnActorFromClass` "/Game/BluePrint/BP_Player.BP_Player_C" (`self.Spawn Transform`) "Undefined" "OverrideRootScale" null null))
  (bind _output_get (set `self.Player` _returnvalue))
  (`/Engine/EditorBlueprintResources/StandardMacros.IsValid` _output_get
    (:`Is Valid`
      _)
    (:`Is Not Valid`
      (`KismetSystemLibrary.PrintString` "create player error")))
  (return))